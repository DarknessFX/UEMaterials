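; BP_Retroreflective is a spotlight actor that feeds retroreflective materials with the light's properties.
; The construction script applies intensity, color, cone angle and radius to the spotlight and matches a scene capture's FOV to the cone, hiding itself from that capture.
; Update writes those values, the actor's position and axes, facing factors and a shadow mask clamp into MPC_Retroreflective, a single shared Material Parameter Collection.
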(fn ConstructionScript
  (bind _spotlightcomponent (Variables|Default|GetSpotLightComponent))
  (Utilities|FlowControl|Sequence
    (:then_0
      (Utilities|Array|Add (Variables|/Script/Engine.SceneCaptureComponent|GetHiddenActors (Variables|Default|GetSceneCaptureComponent2D)) self))
    (:then_1
      (Rendering|Components|Light|SetIntensity _spotlightcomponent (Variables|Default|GetLightIntensity))
      (Rendering|Components|Light|SetLightColor _spotlightcomponent (Variables|Default|GetLightColor) true)
      (Rendering|Lighting|SetOuterConeAngle _spotlightcomponent (Variables|Default|GetLightConeAngle)))
    (:then_2
      (Variables|/Script/Engine.SceneCaptureComponent2D|SetFOVAngle (Variables|Default|GetSceneCaptureComponent2D) (Variables|Default|GetLightConeAngle))
      (Rendering|Lighting|SetAttenuationRadius _spotlightcomponent (Variables|Default|GetLightRadius)))
    (:then_3
      (CallFunction|Update))))

(fn Update
  (Utilities|FlowControl|Sequence
    (:then_0
      (Rendering|Material|SetScalarParameterValue "/Game/Retroreflective/MPC_Retroreflective.MPC_Retroreflective" "LightIntensity" (Variables|Default|GetLightIntensity) :!class /Script/Engine.KismetMaterialLibrary)
      (Rendering|Material|SetScalarParameterValue "/Game/Retroreflective/MPC_Retroreflective.MPC_Retroreflective" "LightConeAngle" (Variables|Default|GetLightConeAngle) :!class /Script/Engine.KismetMaterialLibrary)
      (Rendering|Material|SetScalarParameterValue "/Game/Retroreflective/MPC_Retroreflective.MPC_Retroreflective" "LightRadius" (Variables|Default|GetLightRadius) :!class /Script/Engine.KismetMaterialLibrary)
      (Rendering|Material|SetVectorParameterValue "/Game/Retroreflective/MPC_Retroreflective.MPC_Retroreflective" "LightColor" (Variables|Default|GetLightColor) :!class /Script/Engine.KismetMaterialLibrary))
    (:then_1
      (Rendering|Material|SetVectorParameterValue "/Game/Retroreflective/MPC_Retroreflective.MPC_Retroreflective" "LightPosition" (Math|Conversions|ToLinearColor(Vector) (Transformation|GetActorLocation)) :!class /Script/Engine.KismetMaterialLibrary)
      (Rendering|Material|SetVectorParameterValue "/Game/Retroreflective/MPC_Retroreflective.MPC_Retroreflective" "LightForward" (Math|Conversions|ToLinearColor(Vector) (Transformation|GetActorForwardVector)) :!class /Script/Engine.KismetMaterialLibrary)
      (Rendering|Material|SetVectorParameterValue "/Game/Retroreflective/MPC_Retroreflective.MPC_Retroreflective" "LightUp" (Math|Conversions|ToLinearColor(Vector) (Transformation|GetActorUpVector)) :!class /Script/Engine.KismetMaterialLibrary)
      (Rendering|Material|SetVectorParameterValue "/Game/Retroreflective/MPC_Retroreflective.MPC_Retroreflective" "LightRight" (Math|Conversions|ToLinearColor(Vector) (Transformation|GetActorRightVector)) :!class /Script/Engine.KismetMaterialLibrary))
    (:then_2
      (Rendering|Material|SetScalarParameterValue "/Game/Retroreflective/MPC_Retroreflective.MPC_Retroreflective" "LightFacingFactor" (Variables|LightMaterial|GetLightFacingFactor) :!class /Script/Engine.KismetMaterialLibrary)
      (Rendering|Material|SetScalarParameterValue "/Game/Retroreflective/MPC_Retroreflective.MPC_Retroreflective" "ViewFacingFactor" (Variables|LightMaterial|GetViewFacingFactor) :!class /Script/Engine.KismetMaterialLibrary)
      (Rendering|Material|SetScalarParameterValue "/Game/Retroreflective/MPC_Retroreflective.MPC_Retroreflective" "ShadowMaskClamp" (Variables|LightMaterial|GetShadowMaskClamp) :!class /Script/Engine.KismetMaterialLibrary))))